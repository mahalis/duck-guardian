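; A sibling duck pawn or actor that drifts with its flock through physics impulses on its Body.
; On BeginPlay it gets a random yaw, a slight random roll and a fixed random horizontal wander direction.
; Each tick it applies a delta-scaled impulse blending a pull toward DuckMode's SiblingAveragePosition with that wander direction, weighted toward cohesion.
; GetDesiredMovement returns zero.
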(event EventBeginPlay
  (bind _returnvalue (Math|Random|RandomUnitVector))
  (|CallParentFunction)
  (Transformation|SetWorldRotation (Variables|Default|GetBody) (Math|Rotator|MakeRotator (Math|Random|RandomFloatinRange -2e+01 2e+01) 0.0 (Math|Random|RandomFloatinRange 0.0 3.6e+02)) false true)
  (Variables|Default|SetDesiredMovementDirection (Math|Vector|Normalize (Math|Vector|MakeVector (.x _returnvalue) (.y _returnvalue) 0.0))))

(event EventTick
  (params (DeltaSeconds :type Float%20%28single-precision%29))
  (bind _body (Variables|Default|GetBody))
  (bind _returnvalue (Transformation|GetWorldLocation _body))
  (|CallParentFunction DeltaSeconds)
  (bind _asduck_mode (Utilities|Casting|CastToDuckMode (Game|GetGameMode)))
  (Physics|AddImpulse _body (* (Math|Vector|Lerp(Vector) (* (Math|Vector|Normalize (- (Variables|/Game/Blueprints/DuckMode.DuckMode_C|GetSiblingAveragePosition _asduck_mode) (Math|Vector|MakeVector (.x _returnvalue) (.y _returnvalue) 0.0))) 1.5e+03) (* (Variables|Default|GetDesiredMovementDirection) 3e+03) 0.2) DeltaSeconds) "None" false))

(fn ConstructionScript
  (|CallParentFunction))

(fn GetDesiredMovement
  (return "0, 0, 0"))