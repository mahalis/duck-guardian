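; DuckMode runs a duck-herding game, showing a start screen and focusing the view on the player's YouDuck.
; During play, a cursor trace sets MoveTarget and updates the siblings' average ground-plane position.
; StartGame begins a self-rescheduling timer that spawns SiblingDucks at random spots, while HandleEscape removes escapees with a splash effect.
; Either action input triggers Summon, which quacks and impulses nearby siblings toward YouDuck.
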(event EventBeginPlay
  (bind _outactors (Actor|GetAllActorsOfClass "/Game/Blueprints/YouDuck.YouDuck_C"))
  (bind _output_get (Variables|Default|SetYouDuck (Utilities|Array|Get(acopy) _outactors)))
  (Game|Player|SetViewTargetwithBlend (Game|GetPlayerController 0) _output_get 0.0 "VTBlend_Linear" 0.0 false)
  (Variables|Default|SetMoveTarget (Transformation|GetActorLocation _output_get))
  (bind _outactors_2 (Actor|GetAllActorsOfClass "/Game/Blueprints/SiblingDuck.SiblingDuck_C"))
  (Variables|Default|SetSiblings _outactors_2)
  (CallFunction|ShowStartScreen)
  (Input|SetInputModeGameandUI (Game|GetPlayerController 0) 0 "DoNotLock" false))

(event EventTick
  (params (DeltaSeconds :type Float%20%28single-precision%29))
  (bind _returnvalue (Game|GetPlayerController 0))
  (bind _array (Utilities|Array|MakeArray "ObjectTypeQuery1"))
  (bind _siblings (Variables|Default|GetSiblings))
  (bind (_hitresult _returnvalue_2) (Class|PlayerController|GetHitResultUnderCursorforObjects _returnvalue _array true))
  (if (and (Variables|Default|GetIsPlaying) _returnvalue_2)
    (Variables|Default|SetMoveTarget (.Location (Collision|BreakHitResult _hitresult)))
    ;[1 1 1] sibling average position
    (Variables|Default|SetSiblingAveragePosition "0, 0, 0")
    (for _array_element _siblings
      (Variables|Default|SetSiblingAveragePosition (+ (/ (Math|Vector|MakeVector (.x (Transformation|GetWorldLocation (Variables|/Game/Blueprints/Duck.Duck_C|GetBody _array_element))) (.y (Transformation|GetWorldLocation (Variables|/Game/Blueprints/Duck.Duck_C|GetBody _array_element))) 0.0) (Math|Conversions|ToFloat(Integer) (Utilities|Array|Length _siblings))) (Variables|Default|GetSiblingAveragePosition))))))

(event Input|ActionEvents|InputActionAction1
  (params (Key :type Key%20Structure))
  (:Pressed
    (CallFunction|Summon)))

(event Input|ActionEvents|InputActionAction2
  (params (Key :type Key%20Structure))
  (:Pressed
    (CallFunction|Summon)))

(fn ConstructionScript)

(fn HandleEscape
  (params (Duck :type Sibling%20Duck%20Object%20Reference))
  (Utilities|Array|RemoveItem (Variables|Default|GetSiblings) Duck)
  (Effects|SpawnEmitteratLocation "/Game/Effects/EscapeSplash.EscapeSplash" (Transformation|GetWorldLocation (Variables|/Game/Blueprints/Duck.Duck_C|GetBody Duck))))

(fn ShowStartScreen
  (bind _returnvalue (UserInterface|CreateWidget "/Game/Widgets/StartScreen.StartScreen_C"))
  (UserInterface|Viewport|AddtoViewport _returnvalue 0)
  (Variables|Default|SetGameOver false))

(fn StartGame
  (Variables|Default|SetGameOver false)
  (Variables|Default|SetIsPlaying true)
  (CallFunction|MakeSibling)
  (Input|EnableInput (Game|GetPlayerController 0))
  (Class|WidgetBlueprintLibrary|SetFocustoGameViewport)
  (Input|SetInputModeGameandUI (Game|GetPlayerController 0) 0 "LockAlways" false))

(fn MakeSibling
  (bind _returnvalue (Math|Random|RandomUnitVector))
  (bind _returnvalue_2 (* _returnvalue 2e+02))
  (bind _returnvalue_3 (Game|SpawnActorfromClass "/Game/Blueprints/SiblingDuck.SiblingDuck_C" (Math|Transform|MakeTransform (Math|Vector|MakeVector (.x _returnvalue_2) (.y _returnvalue_2) -4e+01) (Math|Rotator|MakeRotator (Math|Random|RandomFloatinRange -3e+01 3e+01) (Math|Random|RandomFloatinRange -3e+01 3e+01) (Math|Random|RandomFloatinRange 0.0 3.6e+02)) "1,1,1") "Undefined" 0 0))
  (Utilities|Array|Add (Variables|Default|GetSiblings) _returnvalue_3)
  (Utilities|Time|SetTimerbyFunctionName 0 "MakeSibling" 3.0))

(fn Summon
  (bind _youduck (Variables|Default|GetYouDuck))
  (bind _body (Variables|/Game/Blueprints/Duck.Duck_C|GetBody _youduck))
  (bind _returnvalue (Transformation|GetWorldLocation _body))
  (for _array_element (Variables|Default|GetSiblings)
    (if (< (Math|Vector|VectorLength (- _returnvalue (Transformation|GetWorldLocation (Variables|/Game/Blueprints/Duck.Duck_C|GetBody _array_element)))) 5.6e+02)
      (Physics|AddImpulse (Variables|/Game/Blueprints/Duck.Duck_C|GetBody _array_element) (* (Math|Vector|Normalize (- _returnvalue (Transformation|GetWorldLocation (Variables|/Game/Blueprints/Duck.Duck_C|GetBody _array_element)))) 1e+05) "None" false)))
  (Audio|PlaySoundatLocation "/Game/Sounds/Quack.Quack" _returnvalue "0, 0, 0" 1.4))