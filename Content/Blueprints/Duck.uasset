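; Duck actor that floats on a flat water surface at world Z = 0 using simple probe-based buoyancy.
; Each tick, every child of ProbeContainer applies a frame-time-scaled impulse to Body at its location, upward below the surface and weaker downward otherwise.
; Off-center impulses can tilt the body as well as lift it.
; GetDesiredMovement returns a zero vector, so it requests no movement.
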(event EventBeginPlay)

(event EventTick
  (params (DeltaSeconds :type Float%20%28single-precision%29))
  (bind _body (Variables|Default|GetBody))
  ;[1 1 1] buoyancy
  (for _array_element (Components|GetChildrenComponents (Variables|Default|GetProbeContainer) false)
    (if (< (.Z (Math|Vector|BreakVector (Transformation|GetWorldLocation _array_element))) 0.0)
      (Physics|AddImpulseatLocation _body (Math|Vector|MakeVector 0.0 0.0 (* DeltaSeconds 2.2e+04)) (Transformation|GetWorldLocation _array_element) "None")
      (else
        (Physics|AddImpulseatLocation _body (Math|Vector|MakeVector 0.0 0.0 (* DeltaSeconds -8e+03)) (Transformation|GetWorldLocation _array_element) "None")))))

(fn ConstructionScript)

(fn GetDesiredMovement
  (return "0, 0, 0"))