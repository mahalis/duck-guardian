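; YouDuck is a duck actor, apparently the player's, that follows the MoveTarget held by the DuckMode game mode.
; Each tick it eases MovementConstraintActor toward that target with a delta-time-scaled lerp, steering through constraints rather than moving Body directly.
; AngleConstraint's orientation target turns to face the target unless Body is already close to it.
; A line trace for limiting the target to hit points is left disconnected as not fun.
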(event EventBeginPlay
  (|CallParentFunction) ; This node is disabled and will not be called.\nDrag off pins to build functionality.
)

(event Collision|EventActorBeginOverlap
  (params (OtherActor :type Actor%20Object%20Reference))
  (|CallParentFunction OtherActor) ; This node is disabled and will not be called.\nDrag off pins to build functionality.
)

(event EventTick
  (params (DeltaSeconds :type Float%20%28single-precision%29))
  (|CallParentFunction DeltaSeconds)
  (CallFunction|HandleMovement DeltaSeconds))

(fn ConstructionScript
  (|CallParentFunction))

(fn HandleMovement
  (params (A :type Float%20%28single-precision%29))
  (bind _movementconstraintactor (Variables|Default|GetMovementConstraintActor))
  (bind _asduck_mode (Utilities|Casting|CastToDuckMode (Game|GetGameMode)))
  (LocalVariables|SetRestrictedTargetPosition (Variables|/Game/Blueprints/DuckMode.DuckMode_C|GetMoveTarget _asduck_mode)) ; nothing hit; just set the position
  ;[1 1 1] update orientation for target if not too close
  (Transformation|SetActorLocation _movementconstraintactor (Math|Vector|Lerp(Vector) (Transformation|GetActorLocation _movementconstraintactor) (LocalVariables|GetRestrictedTargetPosition) (* A 1.8)) false false)
  (if (> (Math|Vector|VectorLength (- (LocalVariables|GetRestrictedTargetPosition) (Transformation|GetWorldLocation (Variables|Default|GetBody)))) 1e+02)
    (Class|PhysicsConstraintComponent|SetAngularOrientationTarget (Variables|Default|GetAngleConstraint) (Class|KismetMathLibrary|MakeRotfromYZ (Math|Vector|Normalize (- (LocalVariables|GetRestrictedTargetPosition) (Transformation|GetWorldLocation (Variables|Default|GetBody)))) (Math|Vector|MakeVector 0.0 0.0 1.0)))))